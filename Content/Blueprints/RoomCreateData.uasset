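; RoomCreateData holds per-room state during room creation: name, index, room info and the doors and score items added to it.
; Init copies the room's teleport door configs into a spare pool, strips inactive entries in a reverse loop, and records the remaining count.
; Callers draw random spare doors without repeats or fetch the whole pool, optionally clearing it.
; Separate add functions register teleport doors, exit doors and score items.
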(fn `AddExitDoor`
  (params (ExitDoor :type "/Game/Blueprints/InteractionActors/ExitDoor/BP_ExitDoorBase Object Reference (by ref)"))
  (`KismetArrayLibrary.Array_Add` (`self.ExitDoors`) ExitDoor))

(fn `AddScoreItem`
  (params (ScoreItem :type "/Game/Blueprints/InteractionActors/ScoreItem/BP_ScoreItemBase Object Reference (by ref)"))
  (`KismetArrayLibrary.Array_Add` (`self.ScoreItems`) ScoreItem))

(fn `AddTeleportDoor`
  (params (TeleportDoor :type "/Game/Blueprints/InteractionActors/TeleportDoor/BP_TeleportDoorBase Object Reference (by ref)"))
  (`KismetArrayLibrary.Array_Add` (`self.TeleportDoors`) TeleportDoor))

(fn `GetName`
  (returns (Name :type Name))
  (return (`self.Name`)))

(fn `GetRandomTeleportDoorInfo`
  (returns (Succeed :type Boolean) (TeleportDoor :type "/Game/Data/RoomsDT/S_TeleportDoorInfo Structure"))
  (if (`self.IsHaveSpareDoors`)
    (bind _output_get (`self.GetSpareDoorInfo_Random`))
    (return true _output_get)
    (else
      (return false))))

(fn `GetRoomInfo`
  (returns (RoomInfo :type "/Game/Data/RoomsDT/S_RoomInfo Structure"))
  (return (`self.RoomInfo`)))

(fn `GetSpareDoorInfo_Random`
  (returns (Output_Get :type "/Game/Data/RoomsDT/S_TeleportDoorInfo Structure"))
  (locals (SpareDoorInfo :type "/Game/Data/RoomsDT/S_TeleportDoorInfo Structure") (RandomIndex :type Integer :default 0))
  (bind _sparedoorinfos (`self.SpareDoorInfos`))
  (bind _output_get (set `local.RandomIndex` (`KismetMathLibrary.RandomInteger` (`KismetArrayLibrary.Array_Length` _sparedoorinfos))))
  (set `local.SpareDoorInfo` (`|GetArrayItem` _sparedoorinfos _output_get))
  (`KismetArrayLibrary.Array_Remove` _sparedoorinfos (`local.RandomIndex`))
  (return (`local.SpareDoorInfo`)))

(fn `GetSpareDoorInfos`
  (params (Clear :type Boolean))
  (returns (SpareDoorInfos :type "Array of /Game/Data/RoomsDT/S_TeleportDoorInfo Structure"))
  (locals (LocalSpareDoorInfos :type "Array of /Game/Data/RoomsDT/S_TeleportDoorInfo Structure"))
  (bind _sparedoorinfos (`self.SpareDoorInfos`))
  (set `local.LocalSpareDoorInfos` _sparedoorinfos)
  (if Clear
    (`KismetArrayLibrary.Array_Clear` _sparedoorinfos))
  (return (`local.LocalSpareDoorInfos`)))

(fn `GetTeleportDoorsNum`
  (returns (TeleportDoorsNum :type Integer))
  (return (`self.TeleportDoorsNum`)))

(fn `Init`
  (params (Name :type Name) (Index :type Integer) (RoomInfo :type "/Game/Data/RoomsDT/S_RoomInfo Structure"))
  (bind _sparedoorinfos (`self.SpareDoorInfos`))
  (set `self.Name` Name)
  (set `self.Index` Index)
  (bind _output_get (set `self.RoomInfo` RoomInfo))
  (set `self.SpareDoorInfos` (`.TeleportDoors_13_EB7E08BC48D26970CFDBF9818B943375` (break `/Game/Data/RoomsDT/S_RoomInfo` _output_get)))
  (`|ExecutionSequence`
    (:`then_0`
      ;[1 1 1] 移除未激活的配置信息。
      (bind (_arrayindex _arrayelement) (`/Engine/EditorBlueprintResources/StandardMacros.ReverseForEachLoop` _sparedoorinfos)
        (:`LoopBody`
          (if (not (`.ActiveInfo_16_F3C8E4B84583D6C23671DABA0FE4E479` (break `/Game/Data/RoomsDT/S_TeleportDoorInfo` _arrayelement)))
            (`KismetArrayLibrary.Array_Remove` _sparedoorinfos _arrayindex)))))
    (:`then_1`
      (set `self.TeleportDoorsNum` (`KismetArrayLibrary.Array_Length` _sparedoorinfos)))))

(fn `IsHaveSpareDoors`
  (returns (ReturnValue :type Boolean))
  (return (> (`KismetArrayLibrary.Array_Length` (`self.SpareDoorInfos`)) 0)))

(fn `IsHaveTeleportDoors`
  (returns (HaveDoors :type Boolean))
  (return (> (`self.GetTeleportDoorsNum`) 0)))