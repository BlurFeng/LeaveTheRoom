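; Blueprint function library for the main game that gives typed access to core framework objects.
; GetGameState and GetGameMode check validity, then cast to BP_GS_MainGame and BP_GM_MainGame.
; GetCat casts player character 0 to BP_Char_Cat.
; Each function returns a Succeed flag alongside the cast reference, so failed lookups report false.
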(fn `GetCat`
  (returns (Succeed :type Boolean) (`AsBP Char Cat` :type "/Game/Blueprints/BP_Char_Cat Object Reference"))
  (bind _asbp_char_cat (cast `/Game/Blueprints/BP_Char_Cat` (`GameplayStatics.GetPlayerCharacter` null))
    (:`then`
      (return true _asbp_char_cat))
    (:`CastFailed`
      (return false null))))

(fn `GetGameMode`
  (returns (Succeed :type Boolean) (`AsBP GM Main Game` :type "/Game/Blueprints/BP_GM_MainGame Object Reference"))
  (bind _returnvalue (`GameplayStatics.GetGameMode` null))
  (`/Engine/EditorBlueprintResources/StandardMacros.IsValid` _returnvalue
    (:`Is Valid`
      (bind _asbp_gm_main_game (cast `/Game/Blueprints/BP_GM_MainGame` _returnvalue)
        (:`then`
          (return true _asbp_gm_main_game))
        (:`CastFailed`
          _)))
    (:`Is Not Valid`
      _))
  (return false null))

(fn `GetGameState`
  (returns (Succeed :type Boolean) (`AsBP GS Main` :type "/Game/Blueprints/BP_GS_MainGame Object Reference"))
  (bind _returnvalue (`GameplayStatics.GetGameState` null))
  (`/Engine/EditorBlueprintResources/StandardMacros.IsValid` _returnvalue
    (:`Is Valid`
      (bind _asbp_gs_main_game (cast `/Game/Blueprints/BP_GS_MainGame` _returnvalue)
        (:`then`
          (return true _asbp_gs_main_game))
        (:`CastFailed`
          _)))
    (:`Is Not Valid`
      _))
  (return false null))