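; BP_GS_MainGame, by its name the main game's Game State, holds the countdown timer and score.
; TimerReduction lowers the timer, clamped between zero and its total, while ScoreIncrease adds points and ResetData restores both to starting values.
; Getters expose score, time, timer fraction and whether time remains.
; It has no active event logic, so the countdown relies on TimerReduction being called.
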(fn `GetScore`
  (returns (Score :type Integer))
  (return (`self.Score`)))

(fn `GetTimer`
  (returns (Timer :type "Float (double-precision)"))
  (return (`self.Timer`)))

(fn `GetTimerPercent`
  (returns (Percent :type "Float (double-precision)"))
  (return (/ (`self.Timer`) (`self.TimerTotal`))))

(fn `HaveTime`
  (returns (HaveTime :type Boolean))
  (return (> (`self.Timer`) 0.0)))

(fn `IsTimerOver`
  (returns (IsOver :type Boolean))
  (return (<= (`self.Timer`) 0.0)))

(fn `ResetData`
  (`|ExecutionSequence`
    (:`then_0`
      (set `self.Timer` (`KismetMathLibrary.Conv_IntToDouble` (`self.TimerTotal`))))
    (:`then_1`
      (set `self.Score` 0))))

(fn `ScoreIncrease`
  (params (Value :type Integer))
  (set `self.Score` (+ (`self.Score`) Value)))

(fn `TimerReduction`
  (params (Value :type "Float (double-precision)"))
  (set `self.Timer` (`KismetMathLibrary.FClamp` (- (`self.Timer`) Value) 0.0 (`KismetMathLibrary.Conv_IntToDouble` (`self.TimerTotal`)))))

(fn `UserConstructionScript`)