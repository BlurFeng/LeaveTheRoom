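; Base actor for interactable objects, tagged as an interaction actor on BeginPlay and toggled interactive through a NonInteractive gameplay tag.
; It tracks focus and interaction state, with start, over, focus and unfocus calls returning whether state changed.
; Ongoing holds convert elapsed time over HoldNeedTime into clamped progress, calling InteractionProgressCompleted when full.
; Losing focus ends any active interaction, while tap and completion handlers are empty stubs.
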(event `self.ReceiveBeginPlay`
  (`|ExecutionSequence`
    (:`then_0`
      (`self.Init`))))

(fn `Focus`
  (params (interactor :type "Actor Object Reference"))
  (returns (exec :type Boolean))
  (if (`self.IsFocus`)
    (return false)
    (else
      (set `self.IsFocus` true)
      (return true))))

(fn `GetInteractionProgress`
  (returns (Progress :type "Float (double-precision)"))
  (return (`self.InteractionProgress`)))

(fn `Init`
  (`BlueprintGameplayTagLibrary.AddGameplayTag` (`self.GameplayTagContainer`) (struct :`TagName` "EQS.Interaction.Actor")))

(fn `InteractionOngoing`
  (params (interactor :type "Actor Object Reference") (ElapsedSeconds :type "Float (double-precision)"))
  (returns (Exec :type Boolean))
  (bind _holdneedtime (`self.HoldNeedTime`))
  (bind _ininteraction (`self.InInteraction`))
  (`|ExecutionSequence`
    (:`then_0`
      (if _ininteraction
        (`|ExecutionSequence`
          (:`then_0`
            (if (> _holdneedtime 0.0)
              (`self.SetInteractionProgress` interactor (`KismetMathLibrary.FClamp` (/ ElapsedSeconds _holdneedtime))))))))
    (:`then_1`
      (return _ininteraction))))

(fn `InteractionOver`
  (params (interactor :type "Actor Object Reference"))
  (returns (Exec :type Boolean))
  (if (`self.InInteraction`)
    (set `self.InInteraction` false)
    (set `self.InteractionProgress` 0.0)
    (return true)
    (else
      (return false))))

(fn `InteractionProgressCompleted`
  (params (interactor :type "Actor Object Reference")))

(fn `InteractionStarted`
  (params (interactor :type "Actor Object Reference"))
  (returns (Exec :type Boolean))
  (if (`self.InInteraction`)
    (return false)
    (else
      (set `self.InInteraction` true)
      (set `self.InteractionProgress` 0.0)
      (return true))))

(fn `InteractionTap`
  (params (interactor :type "Actor Object Reference")))

(fn `IsInInteraction`
  (returns (InInteraction :type Boolean))
  (return (`self.InInteraction`)))

(fn `SetInteractionProgress`
  (params (interactor :type "Actor Object Reference") (Progress :type "Float (double-precision)"))
  (if (<= (`self.InteractionProgress`) 1.0)
    (bind _output_get (set `self.InteractionProgress` (`KismetMathLibrary.FClamp` Progress)))
    (if (>= _output_get 1.0)
      (`self.InteractionProgressCompleted` interactor))))

(fn `SetInteractive`
  (params (IsInteractive :type Boolean))
  (locals (HaveNonInteractiveTag :type Boolean :default false))
  (bind _gameplaytagcontainer (`self.GameplayTagContainer`))
  (`|ExecutionSequence`
    (:`then_0`
      (set `local.HaveNonInteractiveTag` (`BlueprintGameplayTagLibrary.HasTag` (`self.GameplayTagContainer`) (struct :`TagName` "EQS.Interaction.State.NonInteractive"))))
    (:`then_1`
      (if (== IsInteractive (`local.HaveNonInteractiveTag`))
        (if IsInteractive
          (`BlueprintGameplayTagLibrary.RemoveGameplayTag` _gameplaytagcontainer (struct :`TagName` "EQS.Interaction.State.NonInteractive"))
          (else
            (`BlueprintGameplayTagLibrary.AddGameplayTag` _gameplaytagcontainer (struct :`TagName` "EQS.Interaction.State.NonInteractive"))))))))

(fn `UnFocus`
  (params (interactor :type "Actor Object Reference"))
  (returns (Exec :type Boolean))
  (`|ExecutionSequence`
    (:`then_0`
      (if (`self.InInteraction`)
        (`self.InteractionOver` interactor)))
    (:`then_1`
      (if (`self.IsFocus`)
        (set `self.IsFocus` false)
        (return true)
        (else
          (return false))))))

(fn `UserConstructionScript`)