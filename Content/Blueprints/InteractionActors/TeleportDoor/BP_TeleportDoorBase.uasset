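; Base interaction actor for a teleport door that moves its interactor to a linked door.
; Link stores the target door, and completing the interaction progress teleports the interactor to that door's TeleportPoint location and rotation, if both actor and target are valid.
; Init adds the EQS.Interaction.Actor.TeleportDoor gameplay tag on top of the parent's setup.
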(fn `Init`
  (`parent.Init`)
  (`|ExecutionSequence`
    (:`then_0`
      (`BlueprintGameplayTagLibrary.AddGameplayTag` (`self.GameplayTagContainer`) (struct :`TagName` "EQS.Interaction.Actor.TeleportDoor")))))

(fn `InteractionProgressCompleted`
  (params (interactor :type "Actor Object Reference"))
  (`parent.InteractionProgressCompleted` interactor)
  (`self.TeleportActor` interactor))

(fn `Link`
  (params (TargetTeleportDoor :type "/Game/Blueprints/InteractionActors/TeleportDoor/BP_TeleportDoorBase Object Reference"))
  (set `self.Target Teleport Door` TargetTeleportDoor))

(fn `TeleportActor`
  (params (Actor :type "Actor Object Reference"))
  (bind _target_teleport_door (`self.Target Teleport Door`))
  (bind _teleportpoint (`/Game/Blueprints/InteractionActors/TeleportDoor/BP_TeleportDoorBase.TeleportPoint` _target_teleport_door))
  (`/Engine/EditorBlueprintResources/StandardMacros.IsValid` Actor
    (:`Is Valid`
      (`/Engine/EditorBlueprintResources/StandardMacros.IsValid` _target_teleport_door
        (:`Is Valid`
          (`self.K2_SetActorLocationAndRotation` Actor (`SceneComponent.K2_GetComponentLocation` _teleportpoint) (`SceneComponent.K2_GetComponentRotation` _teleportpoint) false false))))))

(fn `UserConstructionScript`)