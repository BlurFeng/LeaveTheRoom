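; Base exit door actor that ends the game when a character interacts with it after the success condition is met.
; Its Interaction override runs the parent logic, then checks the Succeed flag on the main game mode and calls that game mode's GameOver if it is set.
; The event graph and construction script add no logic of their own.
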(fn `Interaction`
  (params (Character :type "Character Object Reference"))
  (bind (_succeed _asbp_gm_main_game) (`/Game/Blueprints/BP_FL_MainGame.GetGameMode`))
  (`parent.Interaction` Character)
  (if _succeed
    (`/Game/Blueprints/BP_GM_MainGame.GameOver` _asbp_gm_main_game)))

(fn `UserConstructionScript`
  (`parent.UserConstructionScript`))