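; BP_PC_Cat is the cat game's player controller, managing the HUD, interaction prompt and end-of-game screens.
; BeginPlay shows the main widget and sets game-only input.
; OpenUIInteraction lazily creates the prompt, toggles its visibility, resets progress on hide and stores the interaction type (score item, teleport door or exit door), with helpers to read the type and set progress.
; Success and failure functions create their screens once, switch to UI-only input and hide the prompt.
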(event `self.ReceiveBeginPlay`
  (`|ExecutionSequence`
    (:`then_0`
      (bind _returnvalue (`|CreateWidget` "/Game/UMG/UMG_Main.UMG_Main_C"))
      (bind _output_get (set `self.UMG_Main` _returnvalue))
      (`UserWidget.AddToViewport` _output_get 0)
      (`WidgetBlueprintLibrary.SetInputMode_GameOnly` self))))

(fn `GetInteractionActorType`
  (returns (InteractionActorType :type "/Game/Data/RoomsDT/Enum_InteractionActorType Enum"))
  (return (`self.InteractionActorType`)))

(fn `OpenUI_GameFailure`
  (`/Engine/EditorBlueprintResources/StandardMacros.IsValid` (`self.UMG_GameFailure`)
    (:`Is Not Valid`
      (bind _returnvalue (`|CreateWidget` "/Game/UMG/UMG_GameFailure.UMG_GameFailure_C"))
      (bind _output_get (set `self.UMG_GameFailure` _returnvalue))
      (`UserWidget.AddToViewport` _output_get 0)
      (`WidgetBlueprintLibrary.SetInputMode_UIOnlyEx` self _output_get "DoNotLock" true)
      (`self.OpenUI_Interaction` false))))

(fn `OpenUI_GameSuccessUI`
  (`/Engine/EditorBlueprintResources/StandardMacros.IsValid` (`self.UMG_GameSuccess`)
    (:`Is Not Valid`
      (bind _returnvalue (`|CreateWidget` "/Game/UMG/UMG_GameSuccess.UMG_GameSuccess_C"))
      (bind _output_get (set `self.UMG_GameSuccess` _returnvalue))
      (`UserWidget.AddToViewport` _output_get 0)
      (`WidgetBlueprintLibrary.SetInputMode_UIOnlyEx` self _output_get "DoNotLock" true)
      (`self.OpenUI_Interaction` false))))

(fn `OpenUI_Interaction`
  (params (Open :type Boolean) (InteractionType :type "/Game/Data/RoomsDT/Enum_InteractionActorType Enum" :default "NewEnumerator0"))
  (bind _umg_interaction (`self.UMG_Interaction`))
  (`|ExecutionSequence`
    (:`then_0`
      (`/Engine/EditorBlueprintResources/StandardMacros.IsValid` (`self.UMG_Interaction`)
        (:`Is Not Valid`
          (bind _returnvalue (`|CreateWidget` "/Game/UMG/UMG_Interaction.UMG_Interaction_C"))
          (bind _output_get (set `self.UMG_Interaction` _returnvalue))
          (`UserWidget.AddToViewport` _output_get 0))))
    (:`then_1`
      (`|ExecutionSequence`
        (:`then_0`
          (if Open
            (`Widget.SetVisibility` _umg_interaction "Visible")
            (else
              (`Widget.SetVisibility` _umg_interaction "Hidden")
              (`/Game/UMG/UMG_Interaction.SetProgressBar` _umg_interaction 0.0))))
        (:`then_1`
          ;[1 1 1] 1=ScoreItem；2=TeleportDoor；3=ExitDoor；
          (set `self.InteractionActorType` InteractionType))))))

(fn `SetUI_Interaction_Progress`
  (params (Progress :type "Float (double-precision)"))
  (bind _umg_interaction (`self.UMG_Interaction`))
  (`/Engine/EditorBlueprintResources/StandardMacros.IsValid` _umg_interaction
    (:`Is Valid`
      (`/Game/UMG/UMG_Interaction.SetProgressBar` _umg_interaction Progress))))

(fn `UserConstructionScript`)